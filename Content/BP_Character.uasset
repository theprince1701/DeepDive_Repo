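; BP_Character plays a frame-by-frame mesh animation that ripples the water surface as it advances.
; BeginPlay caches the BP_WaterSurface actor, and PlayAnim starts a looping timer at roughly 60 Hz.
; Each tick increments an index and, for valid frames, swaps the StaticMesh from the Frames array, flipbook-style.
; A toggle triggers a water ripple at the actor's location on every other valid frame.
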(event EventBeginPlay
  (bind _returnvalue (Actor|GetActorOfClass "/Game/Effects/Water/Interactive/BP_WaterSurface.BP_WaterSurface_C"))
  (Variables|Default|SetWater _returnvalue))

(fn ConstructionScript)

(fn PlayAnim
  (Utilities|Time|SetTimerbyFunctionName 0 "PlayAnimAtIndex" 0.016667 true))

(fn PlayAnimatIndex
  (Variables|Default|SetIndex (+ (Variables|Default|GetIndex) 1))
  (Utilities|IsValid (Utilities|Array|Get(acopy) (Variables|Default|GetFrames) (Variables|Default|GetIndex))
    (:Is%20Valid
      (Components|StaticMesh|SetStaticMesh (Variables|Default|GetStaticMesh) (Utilities|Array|Get(acopy) (Variables|Default|GetFrames) (Variables|Default|GetIndex)))
      (bind _output_get (Variables|Default|SetPlayWaterSplash (not (Variables|Default|GetPlayWaterSplash))))
      (if _output_get
        (Default|RippleatLocation (Variables|Default|GetWater) (Transformation|GetActorLocation) 1.0)))))