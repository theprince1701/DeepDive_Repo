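; BP_Orb is an orb effect actor that disturbs nearby water and drives a global storm parameter.
; A looping timer started on BeginPlay ripples the level's BP_WaterSurface and spawns Niagara splashes at random nearby points, with splashes placed at world Z zero.
; Tick accumulates elapsed time into StormScale in the water Material Parameter Collection, regardless of activation.
; SetActiv flags the orb active and reveals its extractor beam.
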(event Custom|WaterSplash
  (bind _returnvalue (Transformation|GetActorLocation))
  (bind _returnvalue_2 (Math|Random|RandomUnitVector))
  (bind _returnvalue_3 (* _returnvalue_2 2e+02))
  (bind _returnvalue_4 (+ _returnvalue_3 _returnvalue))
  (bind (_x _y) (Math|Vector|BreakVector _returnvalue_4))
  (Default|RippleatLocation (Variables|Default|GetWater) _returnvalue_4 3.0)
  (Niagara|SpawnSystematLocation "/Game/Effects/Splashes/NS_WaterSplash.NS_WaterSplash" (Math|Vector|MakeVector _x _y 0.0)))

(event EventBeginPlay
  (bind _returnvalue (Actor|GetActorOfClass "/Game/Effects/Water/Interactive/BP_WaterSurface.BP_WaterSurface_C"))
  (Variables|Default|SetWater _returnvalue)
  (Utilities|Time|SetTimerbyEvent (delegate Custom|WaterSplash) 0.45 true))

(event EventTick
  (params (DeltaSeconds :type Float%20%28single-precision%29))
  (if (Variables|Default|GetActiviated)
    _
    (else
      _))
  (bind _output_get (Variables|Default|SetScale (+ DeltaSeconds (Variables|Default|GetScale))))
  (Rendering|Material|SetScalarParameterValue "/Game/Effects/MPC_WaterWorldMaster.MPC_WaterWorldMaster" "StormScale" _output_get :!class /Script/Engine.KismetMaterialLibrary))

(fn ConstructionScript)

(fn SetActiv
  (Variables|Default|SetActiviated true)
  (Rendering|SetVisibility (Variables|Default|GetNS_ExtractorBeam) true false))