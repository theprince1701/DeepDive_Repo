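; Lightning storm actor that periodically strikes surrounding geometry with Niagara bolts.
; On Tick, cooldown-gated random-direction traces spawn a bolt for each hit, then ripple BP_WaterSurface and spawn a splash at the impact.
; EnableVFX shows the extractor beam and starts growing StormScale in the water-world material parameter collection over time.
; CheckForPlayers applies radial damage but is not called within this Blueprint.
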(event Custom|EnableVFX
  (Rendering|SetVisibility (Variables|Default|GetNS_ExtractorBeam) true false)
  (Variables|Default|SetTickCloudOpening true))

(event EventBeginPlay)

(event EventTick
  (params (DeltaSeconds :type Float%20%28single-precision%29))
  (CallFunction|UpdateLightingTraces)
  (if (Variables|Default|GetTickCloudOpening)
    (bind _output_get (Variables|Default|SetScale (+ DeltaSeconds (Variables|Default|GetScale))))
    (Rendering|Material|SetScalarParameterValue "/Game/Effects/MPC_WaterWorldMaster.MPC_WaterWorldMaster" "StormScale" _output_get :!class /Script/Engine.KismetMaterialLibrary)))

(fn ConstructionScript)

(fn UpdateLightingTraces
  (if (>= (- (Utilities|Time|GetTimeSeconds) (Variables|Default|GetLastTrace)) (Variables|Default|GetTraceCooldown))
    (LocalVariables|SetRandomDirection (Math|Random|RandomUnitVector))
    (bind _outhit (Collision|LineTraceByChannel (+ (Transformation|GetActorLocation) (* (LocalVariables|GetRandomDirection) (Variables|Default|GetMinRadius))) (+ (* (LocalVariables|GetRandomDirection) (Variables|Default|GetMaxRadius)) (+ (Transformation|GetActorLocation) (* (LocalVariables|GetRandomDirection) (Variables|Default|GetMinRadius)))) "TraceTypeQuery1" false 0 "None"))
    (Variables|Default|SetLastTrace (Utilities|Time|GetTimeSeconds))
    (if (.bBlockingHit (Collision|BreakHitResult _outhit))
      (bind _returnvalue (Niagara|SpawnSystemAttached "/Game/Effects/Lightning/NS_Lightning.NS_Lightning" (Variables|Default|GetDefaultSceneRoot) "None" "0, 0, 0" "0, 0, 0" "KeepRelativeOffset" true))
      (Utilities|IsValid _returnvalue
        (:Is%20Valid
          (Niagara|SetNiagaraVariable(Vector3) _returnvalue "StartLocation" (+ (Transformation|GetActorLocation) (* (LocalVariables|GetRandomDirection) (Variables|Default|GetMinRadius))))
          (Niagara|SetNiagaraVariable(Vector3) _returnvalue "EndLocation" (+ (.ImpactPoint (Collision|BreakHitResult _outhit)) (* (.ImpactNormal (Collision|BreakHitResult _outhit)) (LocalVariables|GetImpactOffset))))
          (Niagara|SetNiagaraVariable(Vector3) _returnvalue "ImpactNormal" (.ImpactNormal (Collision|BreakHitResult _outhit)))
          (bind _returnvalue_2 (Actor|GetActorOfClass "/Game/Effects/Water/Interactive/BP_WaterSurface.BP_WaterSurface_C"))
          (Default|RippleatLocation _returnvalue_2 (.ImpactPoint (Collision|BreakHitResult _outhit)) 3.0)
          (Niagara|SpawnSystematLocation "/Game/Effects/Splashes/NS_WaterSplash.NS_WaterSplash" (.ImpactPoint (Collision|BreakHitResult _outhit))))))))

(fn CheckforPlayers
  (params (InLocation :type Vector))
  (Game|Damage|ApplyRadialDamage 2e+01 InLocation 4e+02 0 0 (Components|GetOwner) (Pawn|GetController (Game|GetInstigator)) true "ECC_Visibility"))