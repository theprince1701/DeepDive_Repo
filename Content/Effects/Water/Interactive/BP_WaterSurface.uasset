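; Interactive water surface actor that simulates GPU ripples on render targets and feeds height and normal textures to the water material.
; Three height targets rotate in a fixed-rate tick loop, each computed from the previous two, then a normal pass runs.
; A pawn overlapping the box splats movement-scaled force into the current height target.
; Functions also add point ripples, draw shoreline waves and sample height by pixel readback.
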(event OnComponentBeginOverlap(Box)
  (params (OverlappedComponent :type Primitive%20Component%20Object%20Reference) (OtherActor :type Actor%20Object%20Reference) (OtherComp :type Primitive%20Component%20Object%20Reference) (OtherBodyIndex :type Integer) (bFromSweep :type Boolean) (SweepResult :type Hit%20Result%20Structure%20%28by%20ref%29))
  ;[1 1 1] Collision
  ;;[1 1 1] CollisionEnter
  (bind _aspawn (Utilities|Casting|CastToPawn OtherActor))
  (Variables|Default|SetTouchingCharacter _aspawn)
  (Variables|Default|SetLastTouchingActorPosition (Transformation|GetActorLocation _aspawn)))

(event OnComponentEndOverlap(Box)
  (params (OverlappedComponent :type Primitive%20Component%20Object%20Reference) (OtherActor :type Actor%20Object%20Reference) (OtherComp :type Primitive%20Component%20Object%20Reference) (OtherBodyIndex :type Integer))
  ;[1 1 1] Collision
  ;;[1 1 1] CollisionExit
  (Utilities|Casting|CastToPawn OtherActor)
  (Variables|Default|SetTouchingCharacter 0))

(event EventBeginPlay
  ;[1 1 1] Clear RenderTargets on Start
  (Rendering|ClearRenderTarget2D "/Game/Effects/Water/Interactive/RenderTargets/Height0.Height0")
  (Rendering|ClearRenderTarget2D "/Game/Effects/Water/Interactive/RenderTargets/Height1.Height1")
  (Rendering|ClearRenderTarget2D "/Game/Effects/Water/Interactive/RenderTargets/Height2.Height2")
  (Rendering|Material|SetTextureParameterValue (Variables|Default|GetWaterMID) "HeightfieldNormal" "/Game/Effects/Water/Interactive/RenderTargets/HeightNormal.HeightNormal"))

(event EventTick
  (params (DeltaSeconds :type Float%20%28single-precision%29))
  ;[1 1 1] TickWaterSim
  (|UpdatePlayerForces
    (:else
      _)
    (:then
      _))
  (|UpdateTime DeltaSeconds
    (:then
      ;;[1 1 1] UpdateHeightState
      (Variables|Default|SetHeightState (Math|Integer|%(Integer) (+ (Variables|Default|GetHeightState) 1) 3))
      ;;[1 1 1] ComputeHeightSim
      (|ComputerRippleHeightSim))
    (:Completed
      ;;[1 1 1] ComputeNormalSim
      (|ComputeRippleNormals))))

(fn ConstructionScript
  (bind _staticmesh (Variables|Default|GetStaticMesh))
  (Components|StaticMesh|SetStaticMesh (Variables|Default|GetStaticMesh) (Variables|Default|GetWaterMesh))
  (bind _returnvalue (Rendering|Material|CreateDynamicMaterialInstance _staticmesh 0 (Variables|Default|GetWaterMat) "None" :!class /Script/Engine.PrimitiveComponent))
  (Variables|Default|SetWaterMID _returnvalue)
  (Rendering|Material|SetMaterial _staticmesh 0 _returnvalue))

(fn GetHeightRT
  (params (Index :type Integer))
  (if (== Index 0)
    (return "/Game/Effects/Water/Interactive/RenderTargets/Height0.Height0")
    (elif (== Index 1)
      (return "/Game/Effects/Water/Interactive/RenderTargets/Height1.Height1")
      (else
        (return "/Game/Effects/Water/Interactive/RenderTargets/Height2.Height2")))))

(fn GetLastHeight
  (params (HeightIndex :type Integer) (FramesOld :type Integer))
  (bind _heightrt (CallFunction|GetHeightRT (Math|Integer|%(Integer) (+ (- HeightIndex FramesOld) 3) 3)))
  (return _heightrt))

(fn TracefromCamera
  (bind _returnvalue (Game|GetPlayerCameraManager 0))
  (bind _returnvalue_2 (Transformation|GetActorLocation _returnvalue))
  (bind (_outhit _returnvalue_3) (Collision|LineTraceByChannel _returnvalue_2 (+ _returnvalue_2 (* (Math|Vector|Normalize (Math|Rotator|GetRotationXVector (Transformation|GetActorRotation _returnvalue))) (* (Variables|Default|GetInteractionDistance) 1e+01))) "TraceTypeQuery1" false 0 "None"))
  (if _returnvalue_3
    (Utilities|IsValid (.HitActor (Collision|BreakHitResult _outhit)))))

(fn RippleatLocation
  (params (Location :type Vector) (Force :type Float%20%28double-precision%29))
  (bind _staticmesh (Variables|Default|GetStaticMesh))
  ;[1 1 1] DrawRippleAtLocation
  (bind _heightrt (CallFunction|GetHeightRT (Variables|Default|GetHeightState)))
  (bind _returnvalue (Rendering|Material|CreateDynamicMaterialInstance "/Game/Effects/Water/Interactive/M_ForceSplat.M_ForceSplat" "None" "None" :!class /Script/Engine.KismetMaterialLibrary))
  (Rendering|Material|SetVectorParameterValue _returnvalue "ForcePosition" (Math|Conversions|ToLinearColor(Vector) (/ (Math|Transform|TransformLocation (Math|Transform|InvertTransform (Transformation|GetWorldTransform _staticmesh)) Location) (.X (Math|Vector|BreakVector (.Max (Components|StaticMesh|GetLocalBounds _staticmesh)))))) :!class /Script/Engine.MaterialInstanceDynamic)
  (Rendering|Material|SetScalarParameterValue _returnvalue "ForceStrength" Force :!class /Script/Engine.MaterialInstanceDynamic)
  (Rendering|DrawMaterialtoRenderTarget _heightrt _returnvalue))

(fn ShorelineWave
  (params (Direction :type Vector))
  (bind _heightrt (CallFunction|GetHeightRT (Variables|Default|GetHeightState)))
  (bind _returnvalue (Rendering|Material|CreateDynamicMaterialInstance "/Game/Effects/Water/Interactive/ShoreWaves/M_ShoreWave.M_ShoreWave" "None" "None" :!class /Script/Engine.KismetMaterialLibrary))
  (Rendering|Material|SetVectorParameterValue _returnvalue "ForceDirection" (Math|Conversions|ToLinearColor(Vector) Direction) :!class /Script/Engine.MaterialInstanceDynamic)
  (Rendering|Material|SetScalarParameterValue _returnvalue "ForceStrength" 2e+02 :!class /Script/Engine.MaterialInstanceDynamic)
  (Rendering|DrawMaterialtoRenderTarget _heightrt _returnvalue)
  (Utilities|Array|Add (Variables|Default|GetShoreWaves) (Utilities|Struct|MakeSD_ShoreWave 1.0 Direction)))

(fn SampleHeightatLocation
  (params (Location :type Vector))
  (bind _staticmesh (Variables|Default|GetStaticMesh))
  (bind _returnvalue (Transformation|GetWorldTransform _staticmesh))
  (bind _max (Components|StaticMesh|GetLocalBounds _staticmesh))
  (bind _x (Math|Vector|BreakVector _max))
  (bind _returnvalue_2 (Math|Transform|InvertTransform _returnvalue))
  (bind _returnvalue_3 (Math|Transform|TransformLocation _returnvalue_2 Location))
  (bind _returnvalue_4 (/ _returnvalue_3 _x))
  (bind _heightrt (CallFunction|GetHeightRT (Variables|Default|GetHeightState)))
  (bind _returnvalue_5 (Class|KismetRenderingLibrary|ReadRenderTargetPixel _heightrt (Math|Float|Truncate (- 2048.0 (.x _returnvalue_4))) (Math|Float|Truncate (- 2048.0 (.y _returnvalue_4)))))
  (return (Math|Conversions|ToFloat(Byte) (.b _returnvalue_5))))